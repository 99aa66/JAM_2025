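; Character component that drives first-person HUD parallax from how fast the view rotates.
; Each tick it reads pitch and yaw from the owner's camera, or control rotation as fallback, and derives clamped per-frame deltas, wrapping yaw at 180 degrees.
; The smoothed deltas go to the MPC_FP_HUD material parameter collection as ParallaxOffset, alongside the character's location as ActorPosition.
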(event `self.ReceiveBeginPlay`
  (bind _ascharacter (cast `Character` (`self.GetOwner`)))
  (bind _output_get (set `self.Character` _ascharacter))
  (bind _returnvalue (`Actor.GetComponentByClass` _output_get "/Script/Engine.CameraComponent"))
  (`/Engine/EditorBlueprintResources/StandardMacros.IsValid` _returnvalue
    (:`Is Valid`
      (set `self.FirstPersonCamera` _returnvalue))))

(event `self.ReceiveTick`
  (params (DeltaSeconds :type "Float (single-precision)"))
  (bind _character (`self.Character`))
  (`/Engine/EditorBlueprintResources/StandardMacros.IsValid` _character
    (:`Is Valid`
      (`self.UpdateParallax`)
      (`KismetMaterialLibrary.SetVectorParameterValue` "/Game/FirstPersonHUD/MPC_FP_HUD.MPC_FP_HUD" "ActorPosition" (`KismetMathLibrary.Conv_VectorToLinearColor` (`Actor.K2_GetActorLocation` _character))))))

(fn `SetRotationRates`
  (params (Rotation :type "Rotator Structure"))
  (bind _returnvalue (`GameplayStatics.GetWorldDeltaSeconds`))
  (bind _returnvalue_2 (`GameplayStatics.GetWorldDeltaSeconds`))
  (bind _minmaxyaw (`self.MinMaxYaw`))
  (bind (_camerarot_roll _camerarot_pitch _camerarot_yaw) (`KismetMathLibrary.BreakRotator` (`self.CameraRot`)))
  (bind _interpcamratestotargetspeed (`self.InterpCamRatesToTargetSpeed`))
  (bind _interpcamratestozerospeed (`self.InterpCamRatesToZeroSpeed`))
  (bind _minmaxpitch (`self.MinMaxPitch`))
  (bind _returnvalue_3 (- (.yaw Rotation) _camerarot_yaw))
  (set `self.PitchRate` (`KismetMathLibrary.FClamp` (- (.pitch Rotation) _camerarot_pitch) (* _minmaxpitch -1.0) _minmaxpitch))
  (set `self.YawRate` (`KismetMathLibrary.FClamp` (`KismetMathLibrary.SelectFloat` (`KismetMathLibrary.SelectFloat` (- _returnvalue_3 360.0) (+ _returnvalue_3 360.0) (> _returnvalue_3 0.0)) _returnvalue_3 (> (`KismetMathLibrary.Abs` _returnvalue_3) 180.0)) (* _minmaxyaw -1.0) _minmaxyaw))
  (set `self.CameraRot` Rotation)
  ;[1 1 1] Interp to Pitch / Yaw Rates
  (bind _output_get (set `self.PitchParallaxOffset` (`KismetMathLibrary.FInterpTo` (`self.PitchParallaxOffset`) (`self.PitchRate`) _returnvalue _interpcamratestotargetspeed)))
  (bind _output_get_2 (set `self.YawParallaxOffset` (`KismetMathLibrary.FInterpTo` (`self.YawParallaxOffset`) (`self.YawRate`) _returnvalue _interpcamratestotargetspeed)))
  ;[1 1 1] Set Parallax Offset
  (`KismetMaterialLibrary.SetVectorParameterValue` "/Game/FirstPersonHUD/MPC_FP_HUD.MPC_FP_HUD" "ParallaxOffset" (make `LinearColor` _output_get_2 _output_get 0.0 1.0))
  ;[1 1 1] Interp to Zero
  (set `self.PitchRate` (`KismetMathLibrary.FInterpTo` (`self.PitchRate`) 0.0 _returnvalue_2 _interpcamratestozerospeed))
  (set `self.YawRate` (`KismetMathLibrary.FInterpTo` (`self.YawRate`) 0.0 _returnvalue_2 _interpcamratestozerospeed)))

(fn `UpdateParallax`
  (bind _firstpersoncamera (`self.FirstPersonCamera`))
  (`self.SetRotationRates` (`KismetMathLibrary.MakeRotator` 0.0 (.pitch (`KismetMathLibrary.SelectRotator` (`SceneComponent.K2_GetComponentRotation` _firstpersoncamera) (`Pawn.GetControlRotation` (`self.Character`)) (`KismetSystemLibrary.IsValid` _firstpersoncamera))) (+ (.yaw (`KismetMathLibrary.SelectRotator` (`SceneComponent.K2_GetComponentRotation` _firstpersoncamera) (`Pawn.GetControlRotation` (`self.Character`)) (`KismetSystemLibrary.IsValid` _firstpersoncamera))) 180.0))))