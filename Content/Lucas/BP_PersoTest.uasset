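; BP_PersoTest is a test first-person player Blueprint that drives a parallax effect from camera rotation.
; Each Tick adds camera pitch and yaw deltas to clamped rates, which smoothed offsets follow via FInterpTo.
; The offsets go to the ParallaxOffset vector in the Parallax material parameter collection, yaw in R and pitch in G.
; The final interpolation leaves YawRate unchanged, while PitchRate is interpolated from an unset Current input.
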(event `self.ReceiveTick`
  (params (DeltaSeconds :type "Float (single-precision)"))
  (bind _returnvalue (`GameplayStatics.GetWorldDeltaSeconds`))
  (bind _returnvalue_2 (`GameplayStatics.GetWorldDeltaSeconds`))
  (bind (_camerarot_roll _camerarot_pitch _camerarot_yaw) (`KismetMathLibrary.BreakRotator` (`self.CameraRot`)))
  (bind _minmaxpitchrate (`self.MinMaxPitchRate`))
  (bind _minmaxyawrate (`self.MinMaxYawRate`))
  (bind _yawrate (`self.YawRate`))
  (bind _returnvalue_3 (`SceneComponent.K2_GetComponentRotation` (`self.FirstPersonCamera`)))
  (set `self.PitchRate` (`KismetMathLibrary.FClamp` (+ (`self.PitchRate`) (- (.pitch _returnvalue_3) _camerarot_pitch)) (* _minmaxpitchrate -1.0) _minmaxpitchrate))
  (set `self.YawRate` (`KismetMathLibrary.FClamp` (+ (- (.yaw _returnvalue_3) _camerarot_yaw) (`self.YawRate`)) (* _minmaxyawrate -1.0) _minmaxyawrate))
  (set `self.CameraRot` _returnvalue_3)
  (bind _output_get (set `self.PitchParallaxOffset` (`KismetMathLibrary.FInterpTo` (`self.PitchParallaxOffset`) (`self.PitchRate`) _returnvalue_2 5.0)))
  (bind _output_get_2 (set `self.YawParallaxOffset` (`KismetMathLibrary.FInterpTo` (`self.YawParallaxOffset`) (`self.YawRate`) _returnvalue_2 5.0)))
  (`KismetMaterialLibrary.SetVectorParameterValue` "/Game/Lucas/Textures/Parallax.Parallax" "ParallaxOffset" (make `LinearColor` _output_get_2 _output_get 0.0 1.0))
  (set `self.YawRate` (`KismetMathLibrary.FInterpTo` _yawrate _yawrate _returnvalue 5.0))
  (set `self.PitchRate` (`KismetMathLibrary.FInterpTo` 0.0 (`self.PitchRate`) _returnvalue 5.0)))

(fn `UserConstructionScript`)