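; BP_Bulle_Moche is an enemy Blueprint in the Survivors template that customizes its appearance and adds no active gameplay logic of its own.
; After running the parent construction script, it snaps three static mesh components to separate pelvis sockets on the Mesh component.
; Its event graph holds only disabled placeholder events, so any behavior comes from the parent class.
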(fn `UserConstructionScript`
  (`parent.UserConstructionScript`)
  (`SceneComponent.K2_AttachToComponent` (`self.StaticMesh`) (`self.Mesh`) "Bind_Pelvis4Socket_1" "SnapToTarget" "SnapToTarget" "SnapToTarget" true)
  (`SceneComponent.K2_AttachToComponent` (`self.StaticMesh1`) (`self.Mesh`) "Bind_Pelvis4Socket_0" "SnapToTarget" "SnapToTarget" "SnapToTarget" true)
  (`SceneComponent.K2_AttachToComponent` (`self.StaticMesh2`) (`self.Mesh`) "Bind_Pelvis4Socket" "SnapToTarget" "SnapToTarget" "SnapToTarget" true))