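; BP_Bubble_Elec is a bubble actor that shields enemies inside its sphere in the survivors template.
; Sphere overlap begin sets Protected on any BP_Base_Enemy that enters, and overlap end clears it.
; Protection is a plain boolean with no counting, so leaving one bubble clears it even inside another.
; IsAlive reports the inverse of IsDead, and the construction script only calls the parent.
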(event `self.Sphere.OnComponentBeginOverlap`
  (params (OverlappedComponent :type "PrimitiveComponent Object Reference") (OtherActor :type "Actor Object Reference") (OtherComp :type "PrimitiveComponent Object Reference") (OtherBodyIndex :type Integer) (bFromSweep :type Boolean) (SweepResult :type "HitResult Structure (by ref)"))
  (bind _asbp_base_enemy (cast `/Game/SurvivorsTemplate/Blueprints/Enemies/BP_Base_Enemy` OtherActor))
  (set `/Game/SurvivorsTemplate/Blueprints/Enemies/BP_Base_Enemy.Protected?` true _asbp_base_enemy))

(event `self.Sphere.OnComponentEndOverlap`
  (params (OverlappedComponent :type "PrimitiveComponent Object Reference") (OtherActor :type "Actor Object Reference") (OtherComp :type "PrimitiveComponent Object Reference") (OtherBodyIndex :type Integer))
  (bind _asbp_base_enemy (cast `/Game/SurvivorsTemplate/Blueprints/Enemies/BP_Base_Enemy` OtherActor))
  (set `/Game/SurvivorsTemplate/Blueprints/Enemies/BP_Base_Enemy.Protected?` false _asbp_base_enemy))

(fn `IsAlive`
  (returns (IsAlive :type Boolean))
  (return (not (`self.IsDead`))))

(fn `UserConstructionScript`
  (`parent.UserConstructionScript`))