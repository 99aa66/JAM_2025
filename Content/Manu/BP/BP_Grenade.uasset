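; Grenade actor that explodes on the first hit of its static mesh and destroys itself.
; On impact it plays a camera shake and adds a flash-effect widget to the viewport for player 0, regardless of distance.
; A zero-length multi-sphere trace on Visibility, ignoring the player character and drawing debug shapes, applies fixed damage per hit result.
; Damaged actors are added to ActorsToIgnore, which the trace does not read.
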(event `self.StaticMesh.OnComponentHit`
  (params (HitComponent :type "PrimitiveComponent Object Reference") (OtherActor :type "Actor Object Reference") (OtherComp :type "PrimitiveComponent Object Reference") (NormalImpulse :type "Vector Structure") (Hit :type "HitResult Structure (by ref)"))
  (bind (_bblockinghit _binitialoverlap _time _distance _location) (`GameplayStatics.BreakHitResult` Hit))
  (`LegacyCameraShake.StartLegacyCameraShake` (`GameplayStatics.GetPlayerCameraManager` 0) "/Game/Manu/Feedback/CS_Kill_AI.CS_Kill_AI_C")
  (bind _returnvalue (`|CreateWidget` "/Game/Manu/Feedback/W_Flasheffect.W_Flasheffect_C"))
  (`UserWidget.AddToViewport` _returnvalue 0)
  (bind _outhits (`KismetSystemLibrary.SphereTraceMulti` _location _location (`self.Radius`) "TraceTypeQuery1" false (`|MakeArray` (`GameplayStatics.GetPlayerCharacter` 0) :!type "Actor Object Reference") "ForDuration" true (struct :`R` 1.0 :`A` 1.0) (struct :`G` 1.0 :`A` 1.0) 2.0))
  (for _array_element _outhits
    (bind (_bblockinghit_2 _binitialoverlap_2 _time_2 _distance_2 _location_2 _impactpoint _normal _impactnormal _physmat _hitactor) (`GameplayStatics.BreakHitResult` _array_element))
    (`GameplayStatics.ApplyDamage` _hitactor 1.0)
    (`KismetArrayLibrary.Array_Add` (`self.Actors to Ignore`) _hitactor))
  (`self.K2_DestroyActor`))

(fn `UserConstructionScript`)