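; Wave-based enemy spawner manager that fills the level around the first-person player on a looping timer, up to a live enemy cap.
; Setup groups data table rows by allowed wave and starts timers for spawning and wave index increases.
; Each wave picks a random count, then an EQS query around the player supplies locations for random enemies from that wave.
; Spawns chain with short random delays, drawing debug sphere traces at candidate points.
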(event `self.ReceiveBeginPlay`
  (bind _asbp_first_person_character (cast `/Game/FirstPerson/Blueprints/BP_FirstPersonCharacter` (`GameplayStatics.GetPlayerCharacter` 0))
    (:`then`
      (set `self.Player` _asbp_first_person_character)
      (`self.Spawn_Setup`))
    (:`CastFailed`
      (`KismetSystemLibrary.PrintString` "Pas le bon Cast"))))

(event `SpawnWave`
  (`self.Update_Enemy_wave`)
  (set `self.CurrentEnemySpawnIndex` 0)
  (set `self.NumberOfEnemiesToSpawn` (`KismetMathLibrary.RandomIntegerInRange` (`self.MinEnemiesPerWave`) (`self.MaxEnemiesPerWave`)))
  (if (< (`self.Current Enemy Count`) (`self.Max Enemies`)) :!label _label
    (if (< (`self.CurrentEnemySpawnIndex`) (`self.NumberOfEnemiesToSpawn`))
      (`self.FindSpawnLocation`))))

(event `ContinueSpawning`
  (`KismetSystemLibrary.Delay` (`KismetMathLibrary.RandomFloatInRange` 0.05 0.2))
  (goto _label))

(event `DecreaseEnemyCount`
  (`/Engine/EditorBlueprintResources/StandardMacros.DecrementInt` (`self.Current Enemy Count`)
    (:`  `
      (`/Engine/EditorBlueprintResources/StandardMacros.IncrementInt` (`self.Enemies Killed`)))))

(event `IncreaseEnemyCount`
  (`/Engine/EditorBlueprintResources/StandardMacros.IncrementInt` (`self.Current Enemy Count`)))

(fn `FindSpawnLocation`
  (bind _player (`self.Player`))
  (`/Engine/EditorBlueprintResources/StandardMacros.IsValid` _player
    (:`Is Valid`
      (bind _returnvalue (`EnvQueryManager.RunEQSQuery` "/Game/Manu/AI/EQS_FindSpawnPoint.EQS_FindSpawnPoint" _player "AllMatching"))
      (add `EnvQueryInstanceBlueprintWrapper.OnQueryFinishedEvent` _returnvalue (`|CreateDelegate` :!event `Spawn_Enemy`)))))

(fn `Prepare Wave Enemies`
  (for _ (range (+ (`self.Max Game Time`) 1))
    (`KismetArrayLibrary.Array_Add` (`self.EnemySpawn`) (make `/Game/Manu/S-DT/S_EnemySpawns` (`|MakeArray`))))
  (bind _outrownames (`DataTableFunctionLibrary.GetDataTableRowNames` (`self.DT_Enemy_Spawn`)))
  (for _index (range (+ (`KismetArrayLibrary.Array_LastIndex` _outrownames) 1))
    (bind _returnvalue (`|GetDataTableRow` (`self.DT_Enemy_Spawn`) (`|GetArrayItem` _outrownames _index))
      (:`then`
        (`KismetArrayLibrary.Array_Add` (`.Spawns_4_34F2072C401FD12242F66F861F29BE2E` (break `/Game/Manu/S-DT/S_EnemySpawns` (`|GetArrayItem` (`self.EnemySpawn`) (`.Allowed_Wave_12_3774DF7F4371D74C11F88CB1DDE782AC` (break `/Game/Manu/S-DT/S_EnemyType` _returnvalue))))) _returnvalue))))
  (return))

(fn `Spawn_Enemy`
  (params (QueryInstance :type "EnvQueryInstanceBlueprintWrapper Object Reference") (QueryStatus :type "EEnvQueryStatus Enum" :default "Processing"))
  (bind _newvar (`self.NewVar`))
  (bind (_resultlocations _returnvalue) (`EnvQueryInstanceBlueprintWrapper.GetQueryResultsAsLocations` QueryInstance))
  (if _returnvalue
    (for _array_element _newvar
      (`KismetSystemLibrary.SphereTraceSingle` :`Start` _array_element :`End` _array_element :`Radius` 25.0 :`TraceChannel` "TraceTypeQuery1" :`DrawDebugType` "Persistent"))
    (bind _returnvalue_2 (`|SpawnActorFromClass` (`.Enemy_14_AD1876AB466EDD7E8A35AFA1B34045DD` (break `/Game/Manu/S-DT/S_EnemyType` (`KismetArrayLibrary.Array_Random` (`self.Prepared Enemies`)))) (`KismetMathLibrary.MakeTransform` (+ (`KismetArrayLibrary.Array_Random` _newvar) (0.0 0.0 25.0))) "AdjustIfPossibleButAlwaysSpawn" "SelectDefaultAtRuntime" null null))
    (`/Engine/EditorBlueprintResources/StandardMacros.IsValid` _returnvalue_2
      (:`Is Valid`
        (`self.IncreaseEnemyCount`)
        (`/Engine/EditorBlueprintResources/StandardMacros.IncrementInt` (`self.CurrentEnemySpawnIndex`)
          (:`  `
            (`self.ContinueSpawning`)))))
    (else
      (`self.FindSpawnLocation`)
      (`KismetSystemLibrary.PrintString` "ERROR: Did Not Find Spawn Location"))))

(fn `Spawn_Setup`
  (`self.Prepare Wave Enemies`)
  (bind _returnvalue (`KismetSystemLibrary.K2_SetTimer` null "SpawnWave" (`self.SpawnInterval`) true))
  (set `self.SpawnTimerReference` _returnvalue)
  (bind _returnvalue_2 (`KismetSystemLibrary.K2_SetTimer` null "IncreaseWaveIndex" 60.0 true))
  (set `self.PhaseIndexTimer` _returnvalue_2))

(fn `Update_Enemy_wave`
  (bind _spawns (break `/Game/Manu/S-DT/S_EnemySpawns` (`|GetArrayItem` (`self.EnemySpawn`) (`self.Wave index`))))
  (if (`KismetArrayLibrary.Array_IsEmpty` _spawns)
    (return)
    (else
      (set `self.Prepared Enemies` _spawns))))

(fn `UserConstructionScript`)